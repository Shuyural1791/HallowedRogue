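; BP_FloatingText is an actor that shows a floating damage number through a WB_FloatingTextWidget widget component.
; On BeginPlay it writes the truncated Damage value into the widget's text block, and a Fade timeline drives that text's render opacity.
; A Movement timeline lerps the actor upward from its spawn location and destroys it when finished.
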(event EventBeginPlay
  ;[1 1 1] Fade Out
  (Utilities|FlowControl|Sequence
    (:then_0
      (bind _aswb_floating_text_widget (Utilities|Casting|CastToWB_FloatingTextWidget (UserInterface|GetUserWidgetObject (Variables|Default|GetWidget))))
      (Rendering|Components|TextRender|SetText (Variables|/Game/SurvivorsTemplate/Widgets/WB_FloatingTextWidget.WB_FloatingTextWidget_C|GetTextBlock_Damage _aswb_floating_text_widget) (Utilities|Text|ToText(Integer) (Math|Float|Truncate (Variables|Default|GetDamage))))
      (bind _newtrack_0 (Timeline|Fade PlayFromStart)
        (:Update
          (Widget|SetRenderOpacity (Variables|/Game/SurvivorsTemplate/Widgets/WB_FloatingTextWidget.WB_FloatingTextWidget_C|GetTextBlock_Damage _aswb_floating_text_widget) _newtrack_0))))
    (:then_1
      ;[1 1 1] Move Up
      (Variables|Default|SetInitialLocation (Transformation|GetActorLocation))
      (bind _newtrack_0_2 (Timeline|Movement PlayFromStart)
        (:Update
          (Transformation|SetActorLocation (Math|Vector|Lerp(Vector) (Variables|Default|GetInitialLocation) (+ (Variables|Default|GetInitialLocation) "0,0,150.000000") _newtrack_0_2) false false))
        (:Finished
          ;[1 1 1] Destroy when done
          (Actor|DestroyActor))))))

(fn ConstructionScript)